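; BP_OrbitCameraPawn is a pawn that orbits a spring arm camera from player axis input.
; Each tick adds axis values to the spring arm's relative pitch and yaw, clamping pitch to a narrow range and holding roll at zero.
; SetSpringArm sets the arm's length and rotation.
; Tick also prints a debug message on screen every frame.
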(event `self.ReceiveTick`
  (params (DeltaSeconds :type "Float (single-precision)"))
  (bind _springarm (`self.SpringArm`))
  (bind (_relativerotation_roll _relativerotation_pitch _relativerotation_yaw) (`KismetMathLibrary.BreakRotator` (`SceneComponent.RelativeRotation` _springarm)))
  (`SceneComponent.K2_SetRelativeRotation` _springarm (`KismetMathLibrary.MakeRotator` 0.0 (`KismetMathLibrary.FClamp` (+ _relativerotation_pitch (`self.GetInputAxisKeyValue`)) -5.0 30.0) (+ _relativerotation_yaw (`self.GetInputAxisKeyValue`))) false false)
  (`KismetSystemLibrary.PrintString` "ORBIT CAMERA TICKING" true false (struct :`G` 0.66 :`B` 1.0 :`A` 1.0) 1.0))

(fn `SetSpringArm`
  (params (Length :type "Float (double-precision)") (RelativeRotation :type "Rotator Structure"))
  (bind _springarm (`self.SpringArm`))
  (`SceneComponent.K2_SetRelativeRotation` _springarm RelativeRotation false false)
  (set `SpringArmComponent.TargetArmLength` Length _springarm))

(fn `UserConstructionScript`)