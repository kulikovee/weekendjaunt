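; Wing scene component for vehicles that applies aerodynamic lift and drag to an assigned physics body at the component's location.
; Point velocity in local space gives angle of attack, offset by camber, which samples a force curve for coefficients scaled by air density, area and forward speed squared.
; UpdateSync uses world transform, while UpdateAsync composes from a given body transform and reads async-physics velocity.
; Debug lines show forces stored by UpdateSync only.
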(fn `DrawDebugForce`
  (bind _returnvalue (`self.K2_GetComponentLocation`))
  (`KismetSystemLibrary.DrawDebugLine` _returnvalue (+ _returnvalue (`self.DragForce`)) (struct :`R` 1.0 :`A` 1.0) 0.0 2.0)
  (`KismetSystemLibrary.DrawDebugLine` _returnvalue (+ _returnvalue (`self.LiftForce`)) (struct :`B` 1.0 :`A` 1.0) 0.0 2.0))

(fn `SetBody`
  (params (Body :type "PrimitiveComponent Object Reference"))
  (set `self.Body` Body))

(fn `UpdateAsync`
  (params (BodyTransform :type "Transform Structure"))
  (locals (LinearVelocityLocal :type "Vector Structure" :default (0.0 0.0 0.0)) (DragUnitVector :type "Vector Structure" :default (0.0 0.0 0.0)) (LiftUnitVector :type "Vector Structure" :default (0.0 0.0 0.0)) (AngleOfAttack :type "Float (double-precision)" :default 0.0) (HalfRhoAreaVV :type "Float (double-precision)" :default 0.0) (CompTransform :type "Transform Structure") (DragCoeff :type "Float (double-precision)" :default 0.0) (LiftCoeff :type "Float (double-precision)" :default 0.0))
  (bind _body (`self.Body`))
  (bind _halfrhoareavv (`local.HalfRhoAreaVV`))
  (bind _comptransform_location (`KismetMathLibrary.BreakTransform` (`local.CompTransform`)))
  (bind _comptransform (`local.CompTransform`))
  (bind (_linearvelocitylocal_x _linearvelocitylocal_y _linearvelocitylocal_z) (`KismetMathLibrary.BreakVector` (`local.LinearVelocityLocal`)))
  (bind _linearvelocitylocal_x_2 (`KismetMathLibrary.BreakVector` (`local.LinearVelocityLocal`)))
  (bind (_returnvalue_x _returnvalue_y) (`KismetMathLibrary.BreakVector` (`CurveVector.GetVectorValue` (`self.ForceCurve`) (`local.AngleOfAttack`))))
  ;[1 1 1] component world space transform
  (set `local.CompTransform` (`KismetMathLibrary.ComposeTransforms` (`self.GetRelativeTransform`) BodyTransform))
  (`/Engine/EditorBlueprintResources/StandardMacros.IsValid` _body
    (:`Is Valid`
      (bind _returnvalue (`AsyncTickFunctions.ATP_GetLinearVelocityAtPoint` _body (.location _comptransform)))
      (set `local.DragUnitVector` (`KismetMathLibrary.Normal` _returnvalue))
      (set `local.LiftUnitVector` (`KismetMathLibrary.Normal` (`KismetMathLibrary.Cross_VectorVector` (`KismetMathLibrary.GetRightVector` (.rotation _comptransform)) (`local.DragUnitVector`))))
      (set `local.LinearVelocityLocal` (* (`KismetMathLibrary.InverseTransformDirection` _comptransform _returnvalue) 0.01))
      (set `local.AngleOfAttack` (+ (`self.CamberAngle`) (`KismetMathLibrary.DegAtan` (`KismetMathLibrary.SafeDivide` _linearvelocitylocal_z _linearvelocitylocal_x))))
      (set `local.HalfRhoAreaVV` (* 0.5 1.22 (`self.Area`) _linearvelocitylocal_x_2 _linearvelocitylocal_x_2))
      (set `local.DragCoeff` (* _returnvalue_x -1.0))
      (set `local.LiftCoeff` _returnvalue_y)
      (`PrimitiveComponent.AddForceAtLocation` (`self.Body`) (* (+ (* (`local.DragUnitVector`) (* (`local.DragCoeff`) _halfrhoareavv)) (* (`local.LiftUnitVector`) (* (`local.LiftCoeff`) _halfrhoareavv))) 100.0) _comptransform_location "None"))))

(fn `UpdateSync`
  (locals (LinearVelocityLocal :type "Vector Structure" :default (0.0 0.0 0.0)) (DragUnitVector :type "Vector Structure" :default (0.0 0.0 0.0)) (LiftUnitVector :type "Vector Structure" :default (0.0 0.0 0.0)) (AngleOfAttack :type "Float (double-precision)" :default 0.0) (HalfRhoAreaVV :type "Float (double-precision)" :default 0.0) (DragCoeff :type "Float (double-precision)" :default 0.0) (LiftCoeff :type "Float (double-precision)" :default 0.0))
  (bind _returnvalue_location (`KismetMathLibrary.BreakTransform` (`self.K2_GetComponentToWorld`)))
  (bind _returnvalue (`self.K2_GetComponentToWorld`))
  (bind _body (`self.Body`))
  (bind _halfrhoareavv (`local.HalfRhoAreaVV`))
  (bind (_linearvelocitylocal_x _linearvelocitylocal_y _linearvelocitylocal_z) (`KismetMathLibrary.BreakVector` (`local.LinearVelocityLocal`)))
  (bind _linearvelocitylocal_x_2 (`KismetMathLibrary.BreakVector` (`local.LinearVelocityLocal`)))
  (bind (_returnvalue_x _returnvalue_y) (`KismetMathLibrary.BreakVector` (`CurveVector.GetVectorValue` (`self.ForceCurve`) (`local.AngleOfAttack`))))
  (`/Engine/EditorBlueprintResources/StandardMacros.IsValid` _body
    (:`Is Valid`
      (bind _returnvalue_2 (`PrimitiveComponent.GetPhysicsLinearVelocityAtPoint` _body (.location _returnvalue) "None"))
      (set `local.DragUnitVector` (`KismetMathLibrary.Normal` _returnvalue_2))
      (set `local.LiftUnitVector` (`KismetMathLibrary.Normal` (`KismetMathLibrary.Cross_VectorVector` (`KismetMathLibrary.GetRightVector` (.rotation _returnvalue)) (`local.DragUnitVector`))))
      (set `local.LinearVelocityLocal` (* (`KismetMathLibrary.InverseTransformDirection` _returnvalue _returnvalue_2) 0.01))
      (set `local.AngleOfAttack` (+ (`self.CamberAngle`) (`KismetMathLibrary.DegAtan` (`KismetMathLibrary.SafeDivide` _linearvelocitylocal_z _linearvelocitylocal_x))))
      (set `local.HalfRhoAreaVV` (* 0.5 1.22 (`self.Area`) _linearvelocitylocal_x_2 _linearvelocitylocal_x_2))
      (set `local.DragCoeff` (* _returnvalue_x -1.0))
      (set `local.LiftCoeff` _returnvalue_y)
      (set `self.DragForce` (* (`local.DragUnitVector`) (* (`local.DragCoeff`) _halfrhoareavv)))
      (set `self.LiftForce` (* (`local.LiftUnitVector`) (* _halfrhoareavv (`local.LiftCoeff`))))
      (`PrimitiveComponent.AddForceAtLocation` (`self.Body`) (* (+ (`self.DragForce`) (`self.LiftForce`)) 100.0) _returnvalue_location "None"))))